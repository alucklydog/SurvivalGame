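; Survival game mode that handles level startup, game over, restart and quit.
; On BeginPlay it caches the GlobalTimer actor before starting SurvivalGameInstance, so UI created afterwards can bind to the timer, then caches the Storage actor.
; GameOver stops the timer and has the game instance swap all panels for a game-over screen showing the day and hour reached.
; Restart reopens MainLevel and quit runs the exit console command.
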(event Custom|GameOver
  (bind _mygameinstance (Variables|Default|GetMyGameInstance))
  (bind _globaltimer (Variables|Default|GetGlobalTimer))
  (Default|StopTimer (Variables|Default|GetGlobalTimer))
  (Default|隐藏所有面板 (Variables|Default|GetMyGameInstance))
  (Default|创建游戏结束UI _mygameinstance)
  (Default|SetText (Variables|/Game/Blueprints/SurvivalGameInstance.SurvivalGameInstance_C|Get游戏结束面板 _mygameinstance) (Variables|/Game/Blueprints/GlobalTimer.GlobalTimer_C|GetCurrentDay _globaltimer) (Variables|/Game/Blueprints/GlobalTimer.GlobalTimer_C|GetCurrentHour _globaltimer)))

(event Custom|RestartGame
  (Game|OpenLevel(byName) "MainLevel"))

(event Custom|QuitGame
  (Development|ExecuteConsoleCommand "exit" 0))

(event EventBeginPlay
  ;[1 1 1] 先获取GlobalTimer才能创建UI后绑定。
  (Utilities|FlowControl|Sequence
    (:then_0
      (bind _outactors (Actor|GetAllActorsOfClass "/Game/Blueprints/GlobalTimer.GlobalTimer_C"))
      (Variables|Default|SetGlobalTimer (Utilities|Array|Get(acopy) _outactors))
      (bind _assurvival_game_instance (Utilities|Casting|CastToSurvivalGameInstance (Game|GetGameInstance)))
      (Default|GameInstanceBeginPlay _assurvival_game_instance))
    (:then_1
      (bind _outactors_2 (Actor|GetAllActorsOfClass "/Game/Blueprints/Props/Storage.Storage_C"))
      (Variables|Default|SetStorage (Utilities|Array|Get(acopy) _outactors_2)))
    (:then_2
      (Variables|Default|SetMyGameInstance (.AsSurvival%20Game%20Instance (Utilities|Casting|CastToSurvivalGameInstance (Game|GetGameInstance)))))))

(fn ConstructionScript)