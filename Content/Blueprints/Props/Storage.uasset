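; Storage box prop that holds the survival game's items in a Content array of item slots.
; Its Box overlap with the SurvivalCharacter shows or hides the storage UI through the GameInstance and sets a nearby-storage flag on the GameMode.
; Depositing stacks items by Type or appends a new slot; withdrawing takes one unit, based on the passed-in slot's count.
; Both functions broadcast add, count-update or delete events for each change.
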(event OnComponentBeginOverlap(Box)
  (params (OverlappedComponent :type Primitive%20Component%20Object%20Reference) (OtherActor :type Actor%20Object%20Reference) (OtherComp :type Primitive%20Component%20Object%20Reference) (OtherBodyIndex :type Integer) (bFromSweep :type Boolean) (SweepResult :type Hit%20Result%20Structure%20%28by%20ref%29))
  (Utilities|Casting|CastToSurvivalCharacter OtherActor)
  (Default|创建储物箱UI (.AsSurvival%20Game%20Instance (Utilities|Casting|CastToSurvivalGameInstance (Game|GetGameInstance))))
  (Variables|/Game/Blueprints/SurvivalGameMode.SurvivalGameMode_C|Set玩家是否在储物箱附近 (.AsSurvival%20Game%20Mode (Utilities|Casting|CastToSurvivalGameMode (Game|GetGameMode))) true))

(event OnComponentEndOverlap(Box)
  (params (OverlappedComponent :type Primitive%20Component%20Object%20Reference) (OtherActor :type Actor%20Object%20Reference) (OtherComp :type Primitive%20Component%20Object%20Reference) (OtherBodyIndex :type Integer))
  (Utilities|Casting|CastToSurvivalCharacter OtherActor)
  (Default|隐藏储物箱UI (.AsSurvival%20Game%20Instance (Utilities|Casting|CastToSurvivalGameInstance (Game|GetGameInstance))))
  (Variables|/Game/Blueprints/SurvivalGameMode.SurvivalGameMode_C|Set玩家是否在储物箱附近 (.AsSurvival%20Game%20Mode (Utilities|Casting|CastToSurvivalGameMode (Game|GetGameMode))) false))

(event EventBeginPlay)

(event Collision|EventActorBeginOverlap
  (params (OtherActor :type Actor%20Object%20Reference)))

(event EventTick
  (params (DeltaSeconds :type Float%20%28single-precision%29)))

(fn ConstructionScript)

(fn Fun装入物品
  (params (NewItem :type Struct%20Item%20Slot%20Structure))
  (bind (_type _name _icon _count) (Utilities|Struct|BreakStruct_ItemSlot NewItem))
  (for (_array_element _array_index) (Variables|Default|GetContent)
    (if (== _type (.Type (Utilities|Struct|BreakStruct_ItemSlot _array_element)))
      (bind _structout (Utilities|Struct|SetmembersinStruct_ItemSlot (Utilities|Array|Get(acopy) (Variables|Default|GetContent) _array_index) (+ _count (.Count (Utilities|Struct|BreakStruct_ItemSlot _array_element)))))
      (Default|Call更新物品数量 _structout)
      (return)))
  (Utilities|Array|Add (Variables|Default|GetContent) NewItem)
  (Default|Call新增物品 NewItem)
  (return))

(fn Fun取出物品
  (params (RemoveItem :type Struct%20Item%20Slot%20Structure))
  (bind (_type _name _icon _count) (Utilities|Struct|BreakStruct_ItemSlot RemoveItem))
  (bind _returnvalue (- _count 1))
  (for (_array_element _array_index) (Variables|Default|GetContent)
    (if (== _type (.Type (Utilities|Struct|BreakStruct_ItemSlot _array_element)))
      (if (== _returnvalue 0)
        (Default|Call删除物品 RemoveItem)
        (Utilities|Array|RemoveIndex (Variables|Default|GetContent) _array_index)
        (return)
        (else
          (bind _structout (Utilities|Struct|SetmembersinStruct_ItemSlot (Utilities|Array|Get(acopy) (Variables|Default|GetContent) _array_index) _returnvalue))
          (Default|Call更新物品数量 _structout)
          (return))))))