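; Inventory Blueprint that stores item slots in a Content array under a weight-based Capacity limit.
; TestCapacity multiplies the item class's default Weight by the incoming Count and checks the new total against Capacity.
; TryAddItem rejects items that exceed it, otherwise updates CurrentWeight and either increases the count of a same-Type slot or appends one.
; Separate event dispatchers report count changes and new slots, and a boolean returns success.
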(fn TestCapacity
  (params (NewItem :type Struct%20Item%20Slot%20Structure))
  (bind (_type _name _icon _count) (Utilities|Struct|BreakStruct_ItemSlot NewItem))
  (bind _currentweight (Variables|Default|GetCurrentWeight))
  (bind _iteminfo (Utilities|GetClassDefaults _type))
  (bind _weight (Utilities|Struct|BreakStruct_ItemInfo _iteminfo))
  (bind _returnvalue (* _weight _count))
  (bind _returnvalue_2 (+ _returnvalue _currentweight))
  (return (<= _returnvalue_2 (Variables|Default|GetCapacity)) _returnvalue_2))

(fn TryAddItem
  (params (NewItem :type Struct%20Item%20Slot%20Structure))
  (bind (_type _name _icon _count) (Utilities|Struct|BreakStruct_ItemSlot NewItem))
  (bind (_success _nowweight) (CallFunction|TestCapacity NewItem))
  (if _success
    (Variables|Default|SetCurrentWeight _nowweight)
    (for (_array_element _array_index) (Variables|Default|GetContent)
      (if (== (.Type (Utilities|Struct|BreakStruct_ItemSlot _array_element)) _type)
        (bind _structout (Utilities|Struct|SetmembersinStruct_ItemSlot (Utilities|Array|Get(acopy) (Variables|Default|GetContent) _array_index) (.Type (Utilities|Struct|BreakStruct_ItemSlot _array_element)) (.Name (Utilities|Struct|BreakStruct_ItemSlot _array_element)) (.Icon (Utilities|Struct|BreakStruct_ItemSlot _array_element)) (+ (.Count (Utilities|Struct|BreakStruct_ItemSlot _array_element)) _count)))
        (Default|Call背包某物品数量变动 _structout)
        (return true)))
    (Utilities|Array|Add (Variables|Default|GetContent) NewItem)
    (Default|Call背包增加物品 NewItem)
    (return true)
    (else
      (return false))))