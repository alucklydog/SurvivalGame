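; GlobalTimer runs the game's day/night clock, driving the sun and sky from game time.
; Each tick through a gate, it rotates SunLight, updates SkySphere, recaptures SkyLight and derives day, hour and minute, offset a quarter day to start at 06:00.
; Crossing 6:00 or 18:00 fires EnterDay or EnterNight, which message the player's SurvivalCharacter, before IsDayTime updates.
; StopTimer closes the gate, halting these updates.
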(event Custom|EnterDay
  (Default|PrintMessage (.AsSurvival%20Character (Utilities|Casting|CastToSurvivalCharacter (Game|Player|GetPlayerPawn 0))) "天亮了"))

(event Custom|EnterNight
  (Default|PrintMessage (.AsSurvival%20Character (Utilities|Casting|CastToSurvivalCharacter (Game|Player|GetPlayerPawn 0))) "天黑了"))

(event Custom|StopTimer
  (bind _returnvalue (Utilities|Time|GetGameTimeinSeconds))
  (bind _secondsperday (Variables|Default|GetSecondsPerDay))
  (bind _returnvalue_2 (/ _secondsperday 4.0))
  (bind _returnvalue_3 (/ _secondsperday 24.0))
  (bind _returnvalue_4 (+ _returnvalue _returnvalue_2))
  (bind (_remainder _returnvalue_5) (Math|Float|Division(WholeandRemainder) _returnvalue_4 _secondsperday))
  (bind (_remainder_2 _returnvalue_6) (Math|Float|Division(WholeandRemainder) _remainder _returnvalue_3))
  (Utilities|FlowControl|Gate false) ; enters at Close
)

(event EventBeginPlay)

(event Collision|EventActorBeginOverlap
  (params (OtherActor :type Actor%20Object%20Reference)))

(event EventTick
  (params (DeltaSeconds :type Float%20%28single-precision%29))
  (bind _returnvalue (Utilities|Time|GetGameTimeinSeconds))
  (bind _secondsperday (Variables|Default|GetSecondsPerDay))
  (bind _returnvalue_2 (/ _secondsperday 4.0))
  (bind _returnvalue_3 (/ _secondsperday 24.0))
  (bind _returnvalue_4 (+ _returnvalue _returnvalue_2))
  (bind (_remainder _returnvalue_5) (Math|Float|Division(WholeandRemainder) _returnvalue_4 _secondsperday))
  (bind (_remainder_2 _returnvalue_6) (Math|Float|Division(WholeandRemainder) _remainder _returnvalue_3))
  (Utilities|FlowControl|Gate false
    (:Exit
      (Transformation|SetActorRotation (Variables|Default|GetSunLight) (Math|Rotator|MakeRotator 0.0 (|计算太阳角度) 0.0))
      (Default|UpdateSunDirection (Variables|Default|GetSkySphere))
      (Class|SkyLightComponent|RecaptureSky (Variables|/Script/Engine.SkyLight|GetLightComponent (Variables|Default|GetSkyLight)))
      (Variables|Default|SetCurrentDay _returnvalue_5)
      (Variables|Default|SetCurrentHour _returnvalue_6)
      (Variables|Default|SetCurrentMinute (.ReturnValue (Math|Float|Division(WholeandRemainder) _remainder_2 (/ _returnvalue_3 6e+01))))
      (Utilities|FlowControl|Sequence
        (:then_0
          (|昼夜转换事件))
        (:then_1
          (Variables|Default|SetIsDayTime? (and (< (Variables|Default|GetCurrentHour) 18) (>= (Variables|Default|GetCurrentHour) 6))))))))

(fn ConstructionScript)