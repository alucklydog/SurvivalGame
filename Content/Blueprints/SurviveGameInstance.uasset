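; Game instance for a survival game that creates and manages the main HUD widgets.
; It spawns the runtime attribute and time UI once and keeps it on the viewport.
; The pickup panel is created lazily and reused; showing it switches to game-and-UI input with a mouse cursor, and hiding it removes the panel and restores game-only input.
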(event Custom|CreateRunTimeUI
  ;[1 1 1] 创建属性和时间的UI
  (Utilities|IsValid (Variables|Default|GetRunTimeUI)
    (:Is%20Not%20Valid
      (bind _returnvalue (UserInterface|CreateWidget "/Game/UI/RunTime.RunTime_C" (Game|GetPlayerController 0)))
      (bind _output_get (Variables|Default|SetRunTimeUI _returnvalue))
      (UserInterface|Viewport|AddtoViewport _output_get 0))))

(event Custom|CreatePickablePanel
  (bind _returnvalue (Game|GetPlayerController 0))
  ;[1 1 1] 创建拾取面板
  (Utilities|IsValid (Variables|Default|GetPickablePanel)
    (:Is%20Valid
      _)
    (:Is%20Not%20Valid
      (bind _returnvalue_2 (UserInterface|CreateWidget "/Game/UI/PickablePanel.PickablePanel_C" (Game|GetPlayerController 0)))
      (bind _output_get (Variables|Default|SetPickablePanel _returnvalue_2))))
  (UserInterface|Viewport|AddtoViewport _output_get 0)
  (Input|SetInputModeGameandUI _returnvalue (Variables|Default|GetPickablePanel) "DoNotLock" true)
  (Variables|/Script/Engine.PlayerController|SetbShowMouseCursor _returnvalue true))

(event Custom|HidePickablePanel
  (bind _returnvalue (Game|GetPlayerController 0))
  (bind _pickablepanel (Variables|Default|GetPickablePanel))
  (Utilities|IsValid _pickablepanel
    (:Is%20Valid
      (Widget|RemovefromParent _pickablepanel)
      (Input|SetInputModeGameOnly _returnvalue)
      (Variables|/Script/Engine.PlayerController|SetbShowMouseCursor _returnvalue false))))